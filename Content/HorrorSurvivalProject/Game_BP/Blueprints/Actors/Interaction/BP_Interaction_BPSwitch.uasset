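; BP_Interaction_BPSwitch is an interactable switch that turns a referenced LightBP on and off.
; Its Interact event checks that LightBP is valid, then flips the visibility of that object's root component.
; The change does not propagate to child components, so only the root is shown or hidden.
; BeginPlay, overlap and Tick are disabled stubs, and the construction script only calls its parent.
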(event `/Game/HorrorSurvivalProject/Game_BP/Blueprints/Interfaces/BPI_InteractionNEW1.Interact`
  (bind _lightbp (`self.LightBP`))
  (bind _rootcomponent (`Actor.RootComponent` _lightbp))
  (`/Engine/EditorBlueprintResources/StandardMacros.IsValid` _lightbp
    (:`Is Valid`
      (if (`SceneComponent.IsVisible` _rootcomponent)
        (`SceneComponent.SetVisibility` _rootcomponent false false)
        (else
          (`SceneComponent.SetVisibility` _rootcomponent true false))))))

(fn `UserConstructionScript`
  (`parent.UserConstructionScript`))